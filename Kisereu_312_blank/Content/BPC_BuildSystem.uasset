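; BPC_BuildSystem is an unfinished building component for BP_Player, meant to preview placement in build mode.
; BeginPlay caches the player and its first-person camera.
; Disconnected nodes sketch a build-mode toggle and a camera line trace that creates a preview mesh once and moves it to the hit point.
; IA_Build, Tick and PreviewLoop events are empty, so none of that preview logic currently runs.
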(event Custom|Preview%20Loop)

(event Input|EnhancedActionEvents|EnhancedInputActionIA_Build
  (params (ActionValue :type Boolean) (ElapsedSeconds :type Float%20%28double-precision%29) (TriggeredSeconds :type Float%20%28double-precision%29) (InputAction :type Input%20Action%20Object%20Reference :default "/Game/Characters/Actions/IA_Build.IA_Build")))

(event EventBeginPlay
  (bind _asbp_player (Utilities|Casting|CastToBP_Player (Components|GetOwner)))
  (Variables|Default|SetPlayer%20BP _asbp_player)
  (Variables|Default|SetCamera (Variables|/Game/Characters/BP_Player.BP_Player_C|GetFirstPersonCamera _asbp_player)))

(event EventTick
  (params (DeltaSeconds :type Float%20%28single-precision%29)))

(fn ConstructionScript)