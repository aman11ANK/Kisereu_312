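; Base Blueprint for buildable objects, identified by a Tag.
; The construction script looks up buildable data by that Tag through a function library and, when found, applies its mesh to BuildableMesh.
; Interface functions expose the Tag and a socket getter, which returns nothing here.
; The event graph holds no active logic.
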(event EventBeginPlay)

(event Collision|EventActorBeginOverlap
  (params (OtherActor :type Actor%20Object%20Reference)))

(event EventTick
  (params (DeltaSeconds :type Float%20%28single-precision%29)))

(fn ConstructionScript
  (bind _tag (Variables|Default|GetTag))
  (bind (_found_data_ _buildabledata) (CallFunction|FLGetBuildableDatabyTag _tag))
  (if _found_data_
    (Components|StaticMesh|SetStaticMesh (Variables|Default|GetBuildableMesh) (.Mesh (Utilities|Struct|BreakS_BuildableData _buildabledata)))))

(fn IFGetBuildableTag
  (return (Variables|Default|GetTag)))

(fn IFGetSockets
  (return 0))