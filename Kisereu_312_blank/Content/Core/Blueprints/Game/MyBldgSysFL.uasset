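; Blueprint function library for the building system that looks up buildable definitions in DT_BuildableDefintions.
; FLGetBuildableDataByTag uses a gameplay tag's name as the row name and returns the matching row with a found flag.
; FLGetAllBuildableTags walks every row and collects each Tag field into a gameplay tag container.
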(fn FLGetBuildableDatabyTag
  (params (Tag :type Gameplay%20Tag%20Structure))
  (bind _returnvalue (Utilities|GetDataTableRow "/Game/Core/Data/Tables/DT_BuildableDefintions.DT_BuildableDefintions" (GameplayTags|GetTagName Tag))
    (:then
      (return true _returnvalue))))

(fn FLGetAllBuildableTags
  (bind _outrownames (DataTable|GetDataTableRowNames "/Game/Core/Data/Tables/DT_BuildableDefintions.DT_BuildableDefintions"))
  (for _array_element _outrownames
    (bind _returnvalue (Utilities|GetDataTableRow "/Game/Core/Data/Tables/DT_BuildableDefintions.DT_BuildableDefintions" _array_element)
      (:then
        (GameplayTags|AddGameplayTag (LocalVariables|GetBuildableTags%28Local%29) (.Tag (Utilities|Struct|BreakS_BuildableData _returnvalue)) :!class /Script/GameplayTags.BlueprintGameplayTagLibrary))))
  (return (LocalVariables|GetBuildableTags%28Local%29)))