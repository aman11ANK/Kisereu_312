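; BP_Interactable is an interactable resource actor that is used up when Interact is called.
; Interact runs only while IsDepleted is false, subtracting one from ResourceAmount, then overwriting it with the numeric result of a zero-or-below check.
; It then sets IsDepleted to false and destroys the actor with no branch on the amount, so the first interaction removes it.
; The event graph and construction script are empty.
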(event EventBeginPlay)

(event Collision|EventActorBeginOverlap
  (params (OtherActor :type Actor%20Object%20Reference)))

(event EventTick
  (params (DeltaSeconds :type Float%20%28single-precision%29)))

(fn ConstructionScript)

(fn Interact
  (if (not (Variables|Default|GetIsDepleted))
    (Variables|Default|SetResourceAmount (- (Variables|Default|GetResourceAmount) 1.0))
    (Variables|Default|SetResourceAmount (Math|Conversions|ToFloat(Boolean) (<= (Variables|Default|GetResourceAmount) 0.0)))
    (Variables|Default|SetIsDepleted false)
    (Actor|DestroyActor)))