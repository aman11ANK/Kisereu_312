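; BP_ResourceNode is a harvestable resource actor that loses health each time it is interacted with.
; Interact subtracts DamagePerHit from CurrentHealth and, at zero or below, destroys the actor, then broadcasts OnHarvested with the resource type and amount.
; The dispatcher leaves handling of the yield to its listeners.
; The event graph and construction script are empty, so all logic lives in Interact.
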(event EventBeginPlay)

(event Collision|EventActorBeginOverlap
  (params (OtherActor :type Actor%20Object%20Reference)))

(event EventTick
  (params (DeltaSeconds :type Float%20%28single-precision%29)))

(fn ConstructionScript)

(fn Interact
  (Variables|Default|SetCurrentHealth (- (Variables|Default|GetCurrentHealth) (Variables|Default|GetDamagePerHit)))
  (if (<= (Variables|Default|GetCurrentHealth) 0.0)
    (Actor|DestroyActor)
    (Default|CallOnHarvested (Variables|Default|GetResourceType) (Variables|Default|GetResourceAmount))
    (else
      (Variables|Default|SetCurrentHealth (Variables|Default|GetCurrentHealth)))))